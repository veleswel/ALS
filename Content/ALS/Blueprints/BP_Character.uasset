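; Player character Blueprint for an ALS-style locomotion setup, with Enhanced Input for move, look, jump, crouch, aim and hold switching.
; Switching hold links unarmed, one-hand or two-hand anim class layers onto the mesh.
; Aim and crouch change the movement gate, which loads CharacterMovement speed, acceleration and braking from a settings map and notifies the AnimInstance.
; Tick sphere-traces downward and sends ground distance to the AnimInstance.
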(event Input|EnhancedActionEvents|EnhancedInputActionIA_SwitchHold
  (params (ActionValue :type Float%20%28double-precision%29) (ElapsedSeconds :type Float%20%28double-precision%29) (TriggeredSeconds :type Float%20%28double-precision%29) (InputAction :type Input%20Action%20Object%20Reference :default "/Game/ALS/Input/InputActions/IA_SwitchHold.IA_SwitchHold"))
  (bind _mesh (Variables|Character|GetMesh))
  ;[1 1 1 1 14] SwitchHold InputAction
  (:Started
    (switch int (Math|Float|Truncate ActionValue)
      (:1
        (Variables|Default|SetCurrentHandHold "NewEnumerator0")
        (Components|SkeletalMesh|AnimationBlueprintLinking|LinkAnimClassLayers _mesh "/Game/ALS/Blueprints/AnimationBlueprints/LinkedAnimationLayers/ABP_Unarmed.ABP_Unarmed_C"))
      (:2
        (Variables|Default|SetCurrentHandHold "NewEnumerator1")
        (Components|SkeletalMesh|AnimationBlueprintLinking|LinkAnimClassLayers _mesh "/Game/ALS/Blueprints/AnimationBlueprints/LinkedAnimationLayers/ABP_OneHand.ABP_OneHand_C"))
      (:3
        (Variables|Default|SetCurrentHandHold "NewEnumerator2")
        (Components|SkeletalMesh|AnimationBlueprintLinking|LinkAnimClassLayers _mesh "/Game/ALS/Blueprints/AnimationBlueprints/LinkedAnimationLayers/ABP_TwoHand.ABP_TwoHand_C")))))

(event Input|EnhancedActionEvents|EnhancedInputActionIA_Look
  (params (ActionValue :type Vector%202D%20Structure) (ElapsedSeconds :type Float%20%28double-precision%29) (TriggeredSeconds :type Float%20%28double-precision%29) (InputAction :type Input%20Action%20Object%20Reference :default "/Game/ALS/Input/InputActions/IA_Look.IA_Look"))
  ;[1 1 1 1 14] Look InputAction
  (Pawn|Input|AddControllerYawInput (.x ActionValue))
  (Pawn|Input|AddControllerPitchInput (.y ActionValue)))

(event Input|EnhancedActionEvents|EnhancedInputActionIA_Move
  (params (ActionValue :type Vector%202D%20Structure) (ElapsedSeconds :type Float%20%28double-precision%29) (TriggeredSeconds :type Float%20%28double-precision%29) (InputAction :type Input%20Action%20Object%20Reference :default "/Game/ALS/Input/InputActions/IA_Move.IA_Move"))
  (bind _returnvalue (Pawn|GetControlRotation :!class /Script/Engine.Pawn))
  ;[1 1 1 1 14] Move InputAction
  (Pawn|Input|AddMovementInput (Math|Vector|GetRightVector (Math|Rotator|MakeRotator (.roll _returnvalue) 0.0 (.yaw _returnvalue))) (.x ActionValue) false)
  (Pawn|Input|AddMovementInput (Math|Vector|GetForwardVector (Math|Rotator|MakeRotator 0.0 0.0 (.yaw (Pawn|GetControlRotation :!class /Script/Engine.Pawn)))) (.y ActionValue) false))

(event Input|EnhancedActionEvents|EnhancedInputActionIA_Aim
  (params (ActionValue :type Boolean) (ElapsedSeconds :type Float%20%28double-precision%29) (TriggeredSeconds :type Float%20%28double-precision%29) (InputAction :type Input%20Action%20Object%20Reference :default "/Game/ALS/Input/InputActions/IA_Aim.IA_Aim"))
  (:Started
    (Variables|Default|SetIsAiming true)
    (Variables|MovementGate|SetPrevMovementGate (Variables|MovementGate|GetCurrentMovementGate))
    (CallFunction|ApplyMotionGateSetting "NewEnumerator0"))
  (:Completed
    (Variables|Default|SetIsAiming false)
    (Variables|MovementGate|SetPrevMovementGate (Variables|MovementGate|GetCurrentMovementGate))
    (CallFunction|ApplyMotionGateSetting "NewEnumerator1")))

(event Input|EnhancedActionEvents|EnhancedInputActionIA_Crouch
  (params (ActionValue :type Boolean) (ElapsedSeconds :type Float%20%28double-precision%29) (TriggeredSeconds :type Float%20%28double-precision%29) (InputAction :type Input%20Action%20Object%20Reference :default "/Game/ALS/Input/InputActions/IA_Crouch.IA_Crouch"))
  (:Started
    (Variables|Default|SetIsCrouching (not (Variables|Default|GetIsCrouching)))
    (if (Variables|Default|GetIsCrouching)
      (Character|Crouch)
      (Variables|MovementGate|SetPrevMovementGate (Variables|MovementGate|GetCurrentMovementGate))
      (CallFunction|ApplyMotionGateSetting "NewEnumerator2")
      (else
        (Character|UnCrouch)
        (CallFunction|ApplyMotionGateSetting (Variables|MovementGate|GetPrevMovementGate))))))

(event Input|EnhancedActionEvents|EnhancedInputActionIA_Jump
  (params (ActionValue :type Boolean) (ElapsedSeconds :type Float%20%28double-precision%29) (TriggeredSeconds :type Float%20%28double-precision%29) (InputAction :type Input%20Action%20Object%20Reference :default "/Game/ALS/Input/InputActions/IA_Jump.IA_Jump"))
  (:Started
    (Character|Jump))
  (:Completed
    (Character|StopJumping)))

(event EventBeginPlay
  (bind _asplayer_controller (Utilities|Casting|CastToPlayerController (Pawn|GetController)))
  (Input|AddMappingContext (PlayerController|LocalPlayerSubsystems|GetEnhancedInputLocalPlayerSubsystem _asplayer_controller) "/Game/ALS/Input/IMC_Default.IMC_Default" 0 "(bIgnoreAllPressedKeysUntilRelease=True,bForceImmediately=False,bNotifyUserSettings=False)")
  (Components|SkeletalMesh|AnimationBlueprintLinking|LinkAnimClassLayers (Variables|Character|GetMesh) "/Game/ALS/Blueprints/AnimationBlueprints/LinkedAnimationLayers/ABP_Unarmed.ABP_Unarmed_C")
  (CallFunction|ApplyMotionGateSetting "NewEnumerator1")
  (Variables|MovementGate|SetPrevMovementGate "NewEnumerator1"))

(event Collision|EventActorBeginOverlap
  (params (OtherActor :type Actor%20Object%20Reference)))

(event EventTick
  (params (DeltaSeconds :type Float%20%28single-precision%29))
  (bind (_outhit _returnvalue) (Collision|SphereTraceByChannel (- (Transformation|GetActorLocation) (Math|Vector|MakeVector 0.0 0.0 (Variables|/Script/Engine.CapsuleComponent|GetCapsuleHalfHeight (Variables|Collision|GetCapsuleComponent)))) (- (Transformation|GetActorLocation) "0.000000,0.000000,10000.000000") 1.0 "TraceTypeQuery1" false 0 "ForOneFrame"))
  (if _returnvalue
    (Variables|Default|SetDistanceToGround (.Distance (Collision|BreakHitResult _outhit)))
    (Class|BPIAnimationBlueprintIntreface|SetDistancetoGround(Message) (Components|SkeletalMesh|GetAnimInstance (Variables|Character|GetMesh)) (Variables|Default|GetDistanceToGround))))

(fn ConstructionScript)

(fn ApplyMotionGateSetting
  (params (MovementGate :type E_MovementGate%20Enum :default "NewEnumerator0"))
  ;[1 1 1 1 14] Sets CurrentMotionGate and applies corresponding setting to the CharacterMovement
  (bind _output_get (Variables|MovementGate|SetCurrentMovementGate MovementGate))
  (Variables|/Script/Engine.CharacterMovementComponent|SetMaxWalkSpeed (Variables|Character|GetCharacterMovement) (.maxwalkingspeed (.Value (Utilities|Map|Find (Variables|MovementGate|GetMovementGateSettings) _output_get))))
  (Variables|/Script/Engine.CharacterMovementComponent|SetMaxAcceleration (Variables|Character|GetCharacterMovement) (.maxacceleration (.Value (Utilities|Map|Find (Variables|MovementGate|GetMovementGateSettings) _output_get))))
  (Variables|/Script/Engine.CharacterMovementComponent|SetBrakingDecelerationWalking (Variables|Character|GetCharacterMovement) (.brakingdeceleration (.Value (Utilities|Map|Find (Variables|MovementGate|GetMovementGateSettings) _output_get))))
  (Variables|/Script/Engine.CharacterMovementComponent|SetBrakingFriction (Variables|Character|GetCharacterMovement) (.brakingfrictionfactor (.Value (Utilities|Map|Find (Variables|MovementGate|GetMovementGateSettings) _output_get))))
  (Variables|/Script/Engine.CharacterMovementComponent|SetBrakingFrictionFactor (Variables|Character|GetCharacterMovement) (.brakingfriction (.Value (Utilities|Map|Find (Variables|MovementGate|GetMovementGateSettings) _output_get))))
  (Variables|/Script/Engine.CharacterMovementComponent|SetbUseSeparateBrakingFriction (Variables|Character|GetCharacterMovement) (.useseparatebrakingfriction (.Value (Utilities|Map|Find (Variables|MovementGate|GetMovementGateSettings) _output_get))))
  (Class|BPIAnimationBlueprintIntreface|SetCurrentMotionGate(Message) (Components|SkeletalMesh|GetAnimInstance (Variables|Character|GetMesh)) MovementGate))